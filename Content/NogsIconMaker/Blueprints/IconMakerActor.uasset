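; IconMakerActor is a tool actor that renders static mesh icons and exports them as TGA files at 64, 256 and 512 sizes.
; SetMesh assigns the mesh and its first material, and CustomEvent_0 nudges its relative location.
; MakeIcon exports the Small, Medium and Big texture targets selected by its flags.
; Files go to the mesh's own Content folder, named from the asset name after its underscore prefix plus the size.
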(event Custom|Make%20Icon
  (params (64 :type Boolean) (256 :type Boolean) (512 :type Boolean))
  (bind _returnvalue (Class|KismetSystemLibrary|GetProjectDirectory))
  (bind _mesh (Variables|Default|GetMesh))
  (bind _mesh_2 (Variables|Default|GetMesh))
  (bind _staticmesh (Variables|/Script/Engine.StaticMeshComponent|GetStaticMesh _mesh_2))
  (bind _staticmesh_2 (Variables|/Script/Engine.StaticMeshComponent|GetStaticMesh _mesh))
  (bind _returnvalue_2 (Utilities|GetObjectName _staticmesh))
  (bind _returnvalue_3 (Class|KismetSystemLibrary|GetPathName _staticmesh_2))
  (bind _rights (Utilities|String|Split _returnvalue_2 "_"))
  (bind _lefts (Utilities|String|Split _returnvalue_3 "/" "IgnoreCase" "FromEnd"))
  (bind _rights_2 (Utilities|String|Split _lefts "Game/"))
  (bind _returnvalue_4 (Utilities|String|Append _returnvalue "Content/" _rights_2))
  (Utilities|FlowControl|Sequence
    (:then_0
      (if 64
        (Rendering|ExportRenderTarget (Variables|/Script/Engine.SceneCaptureComponent2D|GetTextureTarget (Variables|Default|GetSmall)) _returnvalue_4 (Utilities|String|Append _rights "64.tga"))))
    (:then_1
      (if 256
        (Rendering|ExportRenderTarget (Variables|/Script/Engine.SceneCaptureComponent2D|GetTextureTarget (Variables|Default|GetMedium)) _returnvalue_4 (Utilities|String|Append _rights "256" ".tga"))))
    (:then_2
      (if 512
        (Rendering|ExportRenderTarget (Variables|/Script/Engine.SceneCaptureComponent2D|GetTextureTarget (Variables|Default|GetBig)) _returnvalue_4 (Utilities|String|Append _rights "512.tga"))))))

(event Custom|SetMesh
  (params (NewMesh :type Static%20Mesh%20Object%20Reference))
  (bind _mesh (Variables|Default|GetMesh))
  (Components|StaticMesh|SetStaticMesh _mesh NewMesh)
  (Rendering|Material|SetMaterial _mesh 0 (Rendering|Material|GetMaterial NewMesh 0)))

(event Custom|CustomEvent_0
  (params (B :type Vector))
  (bind _mesh (Variables|Default|GetMesh))
  (Transformation|SetRelativeLocation _mesh (+ (Variables|/Script/Engine.SceneComponent|GetRelativeLocation _mesh) B) false false))

(fn ConstructionScript)